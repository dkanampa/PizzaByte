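; BP_PizzaOrderManager is a game-jam manager actor that holds pizza players, districts and order-frequency curves, mostly as test scaffolding.
; On BeginPlay it spawns dummy players with random funds and nodes, copies districts from the LevelManager after a delay, then stress-tests bankruptcy.
; Tick pushes its players to the GameState.
; The construction script assigns weekday/weekend curves per district type, working around discarded editor defaults; dummy district generation is unused.
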(event EventBeginPlay
  (CallFunction|GenerateDummyPlayers)
  (|CopDistrictsFromLevelManager)
  (|TestBankruptcy))

(event Collision|EventActorBeginOverlap
  (params (OtherActor :type Actor%20Object%20Reference)))

(event EventTick
  (params (DeltaSeconds :type Float%20%28single-precision%29))
  (|GiveGameStateOurPlayers))

(fn ConstructionScript
  (CallFunction|GenerateDefaultCurves))

(fn GenerateDummyDistricts
  (Utilities|Array|Add (Variables|Default|GetDistricts) (Utilities|Struct|MakeDistrict "None" (LocalVariables|GetEmpty%20Sector%20Array) 0 "College" (Utilities|Map|MakeMap "Sausage" 0.5 "Pepperoni" 0.25 "Cheese" 0.15 "Pineapple" 0.1)))
  (Utilities|Array|Add (Variables|Default|GetDistricts) (Utilities|Struct|MakeDistrict "None" (LocalVariables|GetEmpty%20Sector%20Array) 0 "Suburb" (Utilities|Map|MakeMap "Cheese" 0.5 "Pepperoni" 0.25 "Pineapple" 0.15 "Sausage" 0.1)))
  (Utilities|Array|Add (Variables|Default|GetDistricts) (Utilities|Struct|MakeDistrict "None" (LocalVariables|GetEmpty%20Sector%20Array) 0 "Business" (Utilities|Map|MakeMap "Pineapple" 0.5 "Cheese" 0.25 "Pepperoni" 0.15 "Sausage" 0.1))))

(fn GenerateDummyPlayers
  (for _index (range 0 3)
    (bind _returnvalue (Game|SpawnActorfromClass "/Script/GameJam2018_VGDC.PizzaPlayer" (Math|Transform|MakeTransform "0, 0, 0") "Undefined" 0 0))
    (LocalVariables|SetCurrent%20Player _returnvalue)
    (Utilities|FlowControl|Sequence
      (:then_0
        (|GivePlayer$$$))
      (:then_1
        (|SpawnRandom#ofDummyNodes))
      (:then_2
        (|AddPlayertoArray)))))

(fn GenerateDefaultCurves
  ;[1 1 1] UE4 Editor keeps discarding my !@*$ing default curve assignments for this $!@%ing class so we have to use a %(@*ing func
  (Variables|Default|SetOrderFrequencyWeekdays (Utilities|Map|MakeMap "College" "/Game/GameJam/Gameplay/Curves/Curve_2AMMunchieRush.Curve_2AMMunchieRush" "Suburb" "/Game/GameJam/Gameplay/Curves/Curve_DinnerRush.Curve_DinnerRush" "Business" "/Game/GameJam/Gameplay/Curves/Curve_LunchRush.Curve_LunchRush"))
  (Variables|Default|SetOrderFrequencyWeekends (Utilities|Map|MakeMap "College" "/Game/GameJam/Gameplay/Curves/Curve_2AMMunchieRush.Curve_2AMMunchieRush" "Suburb" "/Game/GameJam/Gameplay/Curves/Curve_LunchRush.Curve_LunchRush" "Business" "/Game/GameJam/Gameplay/Curves/Curve_DinnerRush.Curve_DinnerRush")))
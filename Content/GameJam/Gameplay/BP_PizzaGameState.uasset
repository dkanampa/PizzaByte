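; Game state Blueprint that drives the visual day/night cycle through the sky sphere and directional sun light.
; On BeginPlay it builds a period-to-color map and finds the light and sky sphere if unset.
; Each tick it derives sun height from time of day, refreshes the sky material and snaps light color to the current period.
; An older color-blending and intensity-curve path remains disconnected.
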(event EventBeginPlay
  (Utilities|FlowControl|Sequence
    (:then_0
      (|GenerateLightColorMap))
    (:then_1
      (|GetSunLightifnotprovided))
    (:then_2
      (|GetSkySphereifnotprovided))))

(event EventTick
  (params (DeltaSeconds :type Float%20%28single-precision%29))
  (CallFunction|UpdateDayNight))

(fn ConstructionScript)

(fn UpdateDayNight
  (bind _sky_sphere (Variables|Environment|GetSky%20Sphere))
  ;[1 1 1] Update Sky Sphere
  (Variables|/Game/GameJam/Environment/BP_Sky_Sphere_PizzaByte.BP_Sky_Sphere_PizzaByte_C|SetSun%20height _sky_sphere (|Converttimeofdayto[-1,1]))
  (Default|RefreshMaterialFunction _sky_sphere)
  (bind _returnvalue (Class|PizzaGameState|GetPeriodOfDay))
  (Rendering|Components|Light|SetLightColor (Variables|/Script/Engine.Light|GetLightComponent (Variables|Default|GetSunLight)) (.Value (Utilities|Map|Find (Variables|Default|GetLight%20Color%20Map) _returnvalue)) true))
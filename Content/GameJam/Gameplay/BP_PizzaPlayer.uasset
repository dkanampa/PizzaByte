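; BP_PizzaPlayer is the player pawn for a pizza game jam project, providing a drag-to-rotate spring arm camera and spawning the player's UI.
; On BeginPlay it caches its BP_PizzaController, printing an error if the cast fails, then creates the pizza widget for that controller.
; While Rotate Camera is held, look axes apply world yaw and local pitch to the spring arm.
; Each press also refreshes lag speeds from the smoothing settings.
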(event EventBeginPlay
  (CallFunction|FindPizzaController)
  (CallFunction|SpawnUI))

(event Collision|EventActorBeginOverlap
  (params (OtherActor :type Actor%20Object%20Reference)))

(event EventTick
  (params (DeltaSeconds :type Float%20%28single-precision%29)))

(event Input|ActionEvents|InputActionRotateCamera
  (params (Key :type Key%20Structure))
  (:Pressed
    (Variables|Input|SetRotating%20Camera true)
    (|UpdateCameraSmoothing))
  (:Released
    (Variables|Input|SetRotating%20Camera false)))

(event Input|ActionEvents|InputActionSelect
  (params (Key :type Key%20Structure)))

(event Input|AxisEvents|InputAxisLookRight
  (params (AxisValue :type Float%20%28single-precision%29))
  (if (Variables|Input|GetRotating%20Camera)
    (Transformation|AddWorldRotation (Variables|Default|GetCamera%20Spring%20Arm) (Math|Rotator|MakeRotator 0.0 0.0 (* (.X (Math|Vector2D|BreakVector2D (Variables|Input|GetRotation%20Sensitivity))) AxisValue)) false false)))

(event Input|AxisEvents|InputAxisLookUp
  (params (AxisValue :type Float%20%28single-precision%29))
  (if (Variables|Input|GetRotating%20Camera)
    (Transformation|AddLocalRotation (Variables|Default|GetCamera%20Spring%20Arm) (Math|Rotator|MakeRotator 0.0 (* (.Y (Math|Vector2D|BreakVector2D (Variables|Input|GetRotation%20Sensitivity))) AxisValue) 0.0) false false)))

(fn ConstructionScript)

(fn FindPizzaController
  (bind _asbp_pizza_controller (Utilities|Casting|CastToBP_PizzaController (Pawn|GetController))
    (:then
      (Variables|PizzaPlayer|SetPizza%20Player%20Controller _asbp_pizza_controller))
    (:CastFailed
      (Development|PrintString (Utilities|String|Append "##### PLAYER \"" (Utilities|GetDisplayName self) "\" DOES NOT HAVE A BP_PIZZACONTROLLER #####") true true "(R=1.000000,G=0.025664,B=0.000000,A=1.000000)" 15.0))))

(fn SpawnUI
  (bind _returnvalue (UserInterface|CreateWidget "/Game/GameJam/UI/PizzaUi.PizzaUi_C" (Variables|PizzaPlayer|GetPizza%20Player%20Controller)))
  (UserInterface|Viewport|AddtoViewport _returnvalue 0))
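; Level manager actor that holds a nested layout of districts, sectors, blocks and node locations for the game's environment.
; On BeginPlay it adds a scaled box collider at every node and maps each collider to its owning block.
; Tick draws every collider as a debug box.
; An unconnected debug routine can draw nodes as labeled spheres colored by district type.
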(event EventBeginPlay
  (CallFunction|SpawnColliders))

(event Collision|EventActorBeginOverlap
  (params (OtherActor :type Actor%20Object%20Reference)))

(event EventTick
  (params (DeltaSeconds :type Float%20%28single-precision%29))
  (bind _keys (Utilities|Map|Keys (Variables|Default|GetBlockNodeColliders)))
  (for _array_element _keys
    (Rendering|Debug|DrawDebugBox (.Location (Math|Transform|BreakTransform (Transformation|GetWorldTransform _array_element))) (Components|Box|GetScaledBoxExtent _array_element) "(R=0.886515,G=0.327495,B=0.942708,A=1.000000)" "0, 0, 0" 0.0 0.0)))

(fn ConstructionScript)

(fn SpawnColliders
  (for _array_element (Variables|Default|GetDistricts)
    (for _array_element_2 (.Sectors (Utilities|Struct|BreakDistrict _array_element))
      (for _array_element_3 (.Blocks (Utilities|Struct|BreakSector _array_element_2))
        (for _array_element_4 (.NodeLocations (Utilities|Struct|BreakBlock _array_element_3))
          (bind _returnvalue (AddComponent|AddBoxComponent false (Math|Transform|MakeTransform _array_element_4 "0, 0, 0" (Variables|Default|GetColliderScale))))
          (Utilities|Map|Add (Variables|Default|GetBlockNodeColliders) _returnvalue _array_element_3))))))